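; Studio theme controller that applies a selected color and screen theme to the set's monitors and host panels.
; The theme selection picks a DT_Themes row, supplying two colors and a material for each screen.
; Colors go to the MPC_Colors parameter collection, and materials go to valid referenced actors' meshes, with host panels also getting a glossy black slot.
; The same pass runs in the construction script and at BeginPlay.
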(event Custom|GetData
  (bind _returnvalue (Utilities|GetDataTableRow "/Game/Studio/Customize/Themes/DT_Themes.DT_Themes" (Variables|Theme|GetTheme%20Select))
    (:then
      (Variables|Colors|SetColor_1_Selection (.color_01 _returnvalue))
      (Variables|Colors|SetColor_2_Selection (.color_02 _returnvalue))
      (Variables|Monitors|SetOut%20Row%20Monitor%20Front (.monitor_front _returnvalue))
      (Variables|Monitors|SetOut%20Row%20Monitor%20Back (.monitor_back _returnvalue))
      (Variables|Monitors|SetOut%20Row%20Monitor%20Side (.monitor_side _returnvalue))
      (Variables|Panels|SetOut%20Row%20Host%201 (.host_panel_1 _returnvalue))
      (Variables|Panels|SetOut%20Row%20Host%202 (.host_panel_2 _returnvalue))
      (Variables|Panels|SetOut%20Row%20Host%203 (.host_panel_3 _returnvalue))
      (Variables|Panels|SetOut%20Row%20Host%204 (.host_panel_4 _returnvalue))
      (Variables|Panels|SetOut%20Row%20Host%205 (.host_panel_5 _returnvalue)))))

(event Custom|ApplyData
  (Utilities|FlowControl|Sequence
    (:then_0
      (Rendering|Material|SetVectorParameterValue "/Game/Studio/Customize/MPC_Colors.MPC_Colors" "Color1" (Variables|Colors|GetColor_1_Selection) :!class /Script/Engine.KismetMaterialLibrary)
      (Rendering|Material|SetVectorParameterValue "/Game/Studio/Customize/MPC_Colors.MPC_Colors" "Color2" (Variables|Colors|GetColor_2_Selection) :!class /Script/Engine.KismetMaterialLibrary))
    (:then_1
      (bind _monitor_front (Variables|Monitors|GetMonitor_Front)
        (:then
          (Rendering|Material|SetMaterial (Variables|/Game/Assets/Blueprints/BP_MonitorFront.BP_MonitorFront_C|GetSM_Monitor _monitor_front) 0 (Variables|Monitors|GetOut%20Row%20Monitor%20Front)))
        (:else)))
    (:then_2
      (bind _monitor_back (Variables|Monitors|GetMonitor_Back)
        (:then
          (Rendering|Material|SetMaterial (Variables|/Game/Assets/Blueprints/BP_MonitorBack.BP_MonitorBack_C|GetSM_Monitor _monitor_back) 0 (Variables|Monitors|GetOut%20Row%20Monitor%20Back))
          (Variables|Default|SetBlackGlossy "/Game/Assets/Materials/Glossy/MI_Black_Glossy_Pattern.MI_Black_Glossy_Pattern"))
        (:else)))
    (:then_3
      (bind _monitor_side (Variables|Monitors|GetMonitor_Side)
        (:then
          (Rendering|Material|SetMaterial (Variables|/Game/Assets/Blueprints/BP_MonitorSide.BP_MonitorSide_C|GetSM_Monitor _monitor_side) 0 (Variables|Monitors|GetOut%20Row%20Monitor%20Side)))
        (:else)))
    (:then_4
      (bind _host_1 (Variables|Panels|GetHost%201)
        (:then
          (Rendering|Material|SetMaterial (Variables|/Game/Assets/Blueprints/BP_HostPanel_01.BP_HostPanel_01_C|GetSM_Monitor _host_1) 1 (Variables|Panels|GetOut%20Row%20Host%201))
          (Rendering|Material|SetMaterial (Variables|/Game/Assets/Blueprints/BP_HostPanel_01.BP_HostPanel_01_C|GetSM_Monitor _host_1) 0 (Variables|Default|GetBlackGlossy)))
        (:else)))
    (:then_5
      (bind _host_2 (Variables|Panels|GetHost%202)
        (:then
          (Rendering|Material|SetMaterial (Variables|/Game/Assets/Blueprints/BP_HostPanel_02.BP_HostPanel_02_C|GetSM_Monitor _host_2) 1 (Variables|Panels|GetOut%20Row%20Host%202))
          (Rendering|Material|SetMaterial (Variables|/Game/Assets/Blueprints/BP_HostPanel_02.BP_HostPanel_02_C|GetSM_Monitor _host_2) 0 (Variables|Default|GetBlackGlossy)))
        (:else)))
    (:then_6
      (bind _host_3 (Variables|Panels|GetHost%203)
        (:then
          (Rendering|Material|SetMaterial (Variables|/Game/Assets/Blueprints/BP_HostPanel_03.BP_HostPanel_03_C|GetSM_Monitor _host_3) 1 (Variables|Panels|GetOut%20Row%20Host%203))
          (Rendering|Material|SetMaterial (Variables|/Game/Assets/Blueprints/BP_HostPanel_03.BP_HostPanel_03_C|GetSM_Monitor _host_3) 0 (Variables|Default|GetBlackGlossy)))
        (:else)))
    (:then_7
      (bind _host_4 (Variables|Panels|GetHost%204)
        (:then
          (Rendering|Material|SetMaterial (Variables|/Game/Assets/Blueprints/BP_HostPanel_04.BP_HostPanel_04_C|GetSM_Monitor _host_4) 1 (Variables|Panels|GetOut%20Row%20Host%204))
          (Rendering|Material|SetMaterial (Variables|/Game/Assets/Blueprints/BP_HostPanel_04.BP_HostPanel_04_C|GetSM_Monitor _host_4) 0 (Variables|Default|GetBlackGlossy)))
        (:else)))
    (:then_8
      (bind _host_5 (Variables|Panels|GetHost%205)
        (:then
          (Rendering|Material|SetMaterial (Variables|/Game/Assets/Blueprints/BP_HostPanel_05.BP_HostPanel_05_C|GetSM_Monitor _host_5) 1 (Variables|Panels|GetOut%20Row%20Host%205))
          (Rendering|Material|SetMaterial (Variables|/Game/Assets/Blueprints/BP_HostPanel_05.BP_HostPanel_05_C|GetSM_Monitor _host_5) 0 (Variables|Default|GetBlackGlossy)))
        (:else)))))

(event Custom|SetCode
  (Variables|Theme|SetTheme%20Select (Utilities|String|StringToName (Utilities|String|EnumtoString (Variables|Theme|GetThemeSelect)))))

(event EventBeginPlay
  (Utilities|FlowControl|Sequence
    (:then_0
      (CallFunction|SetCode))
    (:then_1
      (CallFunction|GetData)
      (CallFunction|ApplyData))))

(event Collision|EventActorBeginOverlap
  (params (OtherActor :type Actor%20Object%20Reference)))

(event EventTick
  (params (DeltaSeconds :type Float%20%28single-precision%29)))

(fn ConstructionScript
  (Utilities|FlowControl|Sequence
    (:then_0
      (CallFunction|SetCode))
    (:then_1
      (CallFunction|GetData)
      (CallFunction|ApplyData))))