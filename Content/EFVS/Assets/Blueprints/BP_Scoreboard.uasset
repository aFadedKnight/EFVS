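; BP_Scoreboard is an actor that shows leaderboard data fetched from a web URL on its Scoreboard widget component.
; On BeginPlay it sends a VaRest GET request.
; On success it creates a Leaderboard widget, fills only the first row (name, score, wins, elims, placement) from index 1 of the JSON "values" nested array, and assigns it to the component.
; Failure only prints a message.
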(event Custom|Fail
  (params (Request :type Va%20Rest%20Request%20JSON%20Object%20Reference))
  (Development|PrintString "Request Failed"))

(event Custom|Success
  (params (Request :type Va%20Rest%20Request%20JSON%20Object%20Reference))
  (bind _returnvalue (Class|VaRestRequestJSON|GetResponseObject Request))
  (bind _returnvalue_2 (Class|VaRestJsonObject|GetArrayField _returnvalue "values"))
  (bind _output (Utilities|Array|Get(acopy) _returnvalue_2 1))
  (bind _returnvalue_3 (Class|VaRestJsonValue|AsArray _output))
  (Development|PrintString "Success!")
  (bind _returnvalue_4 (UserInterface|CreateWidget "/Game/EFVS/Assets/UMG/Leaderboard.Leaderboard_C"))
  (bind _output_get (Variables|Default|SetLeaderboardReference _returnvalue_4))
  (Default|SetRowOneFields _output_get (Class|VaRestJsonValue|AsString (Utilities|Array|Get(acopy) _returnvalue_3 1)) (Class|VaRestJsonValue|AsString (Utilities|Array|Get(acopy) _returnvalue_3 2)) (Class|VaRestJsonValue|AsString (Utilities|Array|Get(acopy) _returnvalue_3 3)) (Class|VaRestJsonValue|AsString (Utilities|Array|Get(acopy) _returnvalue_3 4)) (Class|VaRestJsonValue|AsString (Utilities|Array|Get(acopy) _returnvalue_3 5)))
  (UserInterface|SetWidget (Variables|Default|GetScoreboard self) _output_get))

(event EventBeginPlay
  (bind _returnvalue (Class|VaRestSubsystem|ConstructVaRestRequestExt (|VaRestSubsystem) "GET" "x_www_form_urlencoded_url"))
  (bind _output_get (Variables|Default|SetRequest _returnvalue))
  (Class|VaRestRequestJSON|SetURL _output_get (Variables|Default|GetURL))
  (EventDispatchers|BindEventtoOnRequestComplete (Variables|Default|GetRequest) (delegate Custom|Success))
  (EventDispatchers|BindEventtoOnRequestFail (Variables|Default|GetRequest) (delegate Custom|Fail))
  (Class|VaRestRequestJSON|ExecuteProcessRequest (Variables|Default|GetRequest)))

(fn ConstructionScript)