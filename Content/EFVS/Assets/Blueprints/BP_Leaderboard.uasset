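; Leaderboard actor that shows player standings on its Scoreboard widget and slides on and off screen.
; On BeginPlay it sends a VaRest GET to a URL, then fills twelve hard-coded rows of a Leaderboard widget from the JSON "values" array.
; ToggleLeaderboard flips the location state, playing a host-nudge level sequence while a timeline lerps the actor between OnScreen and OffScreen.
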(event Custom|Fail
  (params (Request :type Va%20Rest%20Request%20JSON%20Object%20Reference))
  (Development|PrintString "Request Failed"))

(event Custom|Toggle%20Leaderboard
  (if (Utilities|Enum|Equal(Enum) (Variables|Default|GetCurrentLocation) "NewEnumerator5")
    (bind _outactor (Sequencer|Player|CreateLevelSequencePlayer "/Game/EFVS/Studio/LevelSequences/Extra/LS_NudgeHostsCenter_R.LS_NudgeHostsCenter_R"))
    (Sequencer|Player|Play (Variables|/Script/LevelSequence.LevelSequenceActor|GetSequencePlayer _outactor) :!class /Script/MovieScene.MovieSceneSequencePlayer)
    (Utilities|FlowControl|Sequence
      (:then_0
        (bind _logomove (Timeline|Timeline_1 PlayFromStart)
          (:Update
            (Transformation|SetActorLocation (Math|Vector|Lerp(Vector) (Variables|Default|GetOnScreen) (Variables|Default|GetOffScreen) _logomove) false false)
            (Variables|Default|SetCurrentLocation "NewEnumerator6")))))
    (else
      (bind _outactor_2 (Sequencer|Player|CreateLevelSequencePlayer "/Game/EFVS/Studio/LevelSequences/Extra/LS_NudgeHostsRight.LS_NudgeHostsRight"))
      (Sequencer|Player|Play (Variables|/Script/LevelSequence.LevelSequenceActor|GetSequencePlayer _outactor_2) :!class /Script/MovieScene.MovieSceneSequencePlayer)
      (Utilities|FlowControl|Sequence
        (:then_0
          (bind _logomove_2 (Timeline|Timeline_0 PlayFromStart)
            (:Update
              (Transformation|SetActorLocation (Math|Vector|Lerp(Vector) (Variables|Default|GetOffScreen) (Variables|Default|GetOnScreen) _logomove_2) false false)
              (Variables|Default|SetCurrentLocation "NewEnumerator5"))))))))

(event Custom|Success
  (params (Request :type Va%20Rest%20Request%20JSON%20Object%20Reference))
  (bind _returnvalue (Class|VaRestRequestJSON|GetResponseObject Request))
  (bind _returnvalue_2 (Class|VaRestJsonObject|GetArrayField _returnvalue "values"))
  (bind _output (Utilities|Array|Get(acopy) _returnvalue_2 13))
  (bind _output_2 (Utilities|Array|Get(acopy) _returnvalue_2 12))
  (bind _output_3 (Utilities|Array|Get(acopy) _returnvalue_2 11))
  (bind _output_4 (Utilities|Array|Get(acopy) _returnvalue_2 8))
  (bind _output_5 (Utilities|Array|Get(acopy) _returnvalue_2 9))
  (bind _output_6 (Utilities|Array|Get(acopy) _returnvalue_2 10))
  (bind _output_7 (Utilities|Array|Get(acopy) _returnvalue_2 2))
  (bind _output_8 (Utilities|Array|Get(acopy) _returnvalue_2 3))
  (bind _output_9 (Utilities|Array|Get(acopy) _returnvalue_2 4))
  (bind _output_10 (Utilities|Array|Get(acopy) _returnvalue_2 5))
  (bind _output_11 (Utilities|Array|Get(acopy) _returnvalue_2 6))
  (bind _output_12 (Utilities|Array|Get(acopy) _returnvalue_2 7))
  (bind _returnvalue_3 (Class|VaRestJsonValue|AsArray _output_4))
  (bind _returnvalue_4 (Class|VaRestJsonValue|AsArray _output_5))
  (bind _returnvalue_5 (Class|VaRestJsonValue|AsArray _output_6))
  (bind _returnvalue_6 (Class|VaRestJsonValue|AsArray _output_7))
  (bind _returnvalue_7 (Class|VaRestJsonValue|AsArray _output_8))
  (bind _returnvalue_8 (Class|VaRestJsonValue|AsArray _output_9))
  (bind _returnvalue_9 (Class|VaRestJsonValue|AsArray _output_10))
  (bind _returnvalue_10 (Class|VaRestJsonValue|AsArray _output_11))
  (bind _returnvalue_11 (Class|VaRestJsonValue|AsArray _output_12))
  (bind _returnvalue_12 (Class|VaRestJsonValue|AsArray _output_3))
  (bind _returnvalue_13 (Class|VaRestJsonValue|AsArray _output_2))
  (bind _returnvalue_14 (Class|VaRestJsonValue|AsArray _output))
  (Development|PrintString "Success!")
  (bind _returnvalue_15 (UserInterface|CreateWidget "/Game/EFVS/Assets/UMG/Leaderboard.Leaderboard_C"))
  (bind _output_get (Variables|Default|SetLeaderboardReference _returnvalue_15))
  (Utilities|FlowControl|Sequence
    (:then_0
      (Default|SetRowOneFields _output_get (Class|VaRestJsonValue|AsString (Utilities|Array|Get(acopy) _returnvalue_6 1)) (Class|VaRestJsonValue|AsString (Utilities|Array|Get(acopy) _returnvalue_6 2)) (Class|VaRestJsonValue|AsString (Utilities|Array|Get(acopy) _returnvalue_6 3)) (Class|VaRestJsonValue|AsString (Utilities|Array|Get(acopy) _returnvalue_6 4)) (Class|VaRestJsonValue|AsString (Utilities|Array|Get(acopy) _returnvalue_6 5)))
      (UserInterface|SetWidget (Variables|Default|GetScoreboard) _output_get :!label _label))
    (:then_1
      (Default|SetRowTwoFields _output_get (Class|VaRestJsonValue|AsString (Utilities|Array|Get(acopy) _returnvalue_7 1)) (Class|VaRestJsonValue|AsString (Utilities|Array|Get(acopy) _returnvalue_7 2)) (Class|VaRestJsonValue|AsString (Utilities|Array|Get(acopy) _returnvalue_7 3)) (Class|VaRestJsonValue|AsString (Utilities|Array|Get(acopy) _returnvalue_7 4)) (Class|VaRestJsonValue|AsString (Utilities|Array|Get(acopy) _returnvalue_7 5)))
      (goto _label))
    (:then_2
      (Default|SetRowThreeFields _output_get (Class|VaRestJsonValue|AsString (Utilities|Array|Get(acopy) _returnvalue_8 1)) (Class|VaRestJsonValue|AsString (Utilities|Array|Get(acopy) _returnvalue_8 2)) (Class|VaRestJsonValue|AsString (Utilities|Array|Get(acopy) _returnvalue_8 3)) (Class|VaRestJsonValue|AsString (Utilities|Array|Get(acopy) _returnvalue_8 4)) (Class|VaRestJsonValue|AsString (Utilities|Array|Get(acopy) _returnvalue_8 5)))
      (goto _label))
    (:then_3
      (Default|SetRowFourFields _output_get (Class|VaRestJsonValue|AsString (Utilities|Array|Get(acopy) _returnvalue_9 1)) (Class|VaRestJsonValue|AsString (Utilities|Array|Get(acopy) _returnvalue_9 2)) (Class|VaRestJsonValue|AsString (Utilities|Array|Get(acopy) _returnvalue_9 3)) (Class|VaRestJsonValue|AsString (Utilities|Array|Get(acopy) _returnvalue_9 4)) (Class|VaRestJsonValue|AsString (Utilities|Array|Get(acopy) _returnvalue_9 5))))
    (:then_4
      (Default|SetRowFiveFields _output_get (Class|VaRestJsonValue|AsString (Utilities|Array|Get(acopy) _returnvalue_10 1)) (Class|VaRestJsonValue|AsString (Utilities|Array|Get(acopy) _returnvalue_10 2)) (Class|VaRestJsonValue|AsString (Utilities|Array|Get(acopy) _returnvalue_10 3)) (Class|VaRestJsonValue|AsString (Utilities|Array|Get(acopy) _returnvalue_10 4)) (Class|VaRestJsonValue|AsString (Utilities|Array|Get(acopy) _returnvalue_10 5))))
    (:then_5
      (Default|SetRowSixFields _output_get (Class|VaRestJsonValue|AsString (Utilities|Array|Get(acopy) _returnvalue_11 1)) (Class|VaRestJsonValue|AsString (Utilities|Array|Get(acopy) _returnvalue_11 2)) (Class|VaRestJsonValue|AsString (Utilities|Array|Get(acopy) _returnvalue_11 3)) (Class|VaRestJsonValue|AsString (Utilities|Array|Get(acopy) _returnvalue_11 4)) (Class|VaRestJsonValue|AsString (Utilities|Array|Get(acopy) _returnvalue_11 5))))
    (:then_6
      (Default|SetRowSevenFields _output_get (Class|VaRestJsonValue|AsString (Utilities|Array|Get(acopy) _returnvalue_3 1)) (Class|VaRestJsonValue|AsString (Utilities|Array|Get(acopy) _returnvalue_3 2)) (Class|VaRestJsonValue|AsString (Utilities|Array|Get(acopy) _returnvalue_3 3)) (Class|VaRestJsonValue|AsString (Utilities|Array|Get(acopy) _returnvalue_3 4)) (Class|VaRestJsonValue|AsString (Utilities|Array|Get(acopy) _returnvalue_3 5))))
    (:then_7
      (Default|SetRowEightFields _output_get (Class|VaRestJsonValue|AsString (Utilities|Array|Get(acopy) _returnvalue_4 1)) (Class|VaRestJsonValue|AsString (Utilities|Array|Get(acopy) _returnvalue_4 2)) (Class|VaRestJsonValue|AsString (Utilities|Array|Get(acopy) _returnvalue_4 3)) (Class|VaRestJsonValue|AsString (Utilities|Array|Get(acopy) _returnvalue_4 4)) (Class|VaRestJsonValue|AsString (Utilities|Array|Get(acopy) _returnvalue_4 5))))
    (:then_8
      (Default|SetRowNineFields _output_get (Class|VaRestJsonValue|AsString (Utilities|Array|Get(acopy) _returnvalue_5 1)) (Class|VaRestJsonValue|AsString (Utilities|Array|Get(acopy) _returnvalue_5 2)) (Class|VaRestJsonValue|AsString (Utilities|Array|Get(acopy) _returnvalue_5 3)) (Class|VaRestJsonValue|AsString (Utilities|Array|Get(acopy) _returnvalue_5 4)) (Class|VaRestJsonValue|AsString (Utilities|Array|Get(acopy) _returnvalue_5 5))))
    (:then_9
      (Default|SetRowTenFields _output_get (Class|VaRestJsonValue|AsString (Utilities|Array|Get(acopy) _returnvalue_12 1)) (Class|VaRestJsonValue|AsString (Utilities|Array|Get(acopy) _returnvalue_12 2)) (Class|VaRestJsonValue|AsString (Utilities|Array|Get(acopy) _returnvalue_12 3)) (Class|VaRestJsonValue|AsString (Utilities|Array|Get(acopy) _returnvalue_12 4)) (Class|VaRestJsonValue|AsString (Utilities|Array|Get(acopy) _returnvalue_12 5))))
    (:then_10
      (Default|SetRowElevenFields _output_get (Class|VaRestJsonValue|AsString (Utilities|Array|Get(acopy) _returnvalue_13 1)) (Class|VaRestJsonValue|AsString (Utilities|Array|Get(acopy) _returnvalue_13 2)) (Class|VaRestJsonValue|AsString (Utilities|Array|Get(acopy) _returnvalue_13 3)) (Class|VaRestJsonValue|AsString (Utilities|Array|Get(acopy) _returnvalue_13 4)) (Class|VaRestJsonValue|AsString (Utilities|Array|Get(acopy) _returnvalue_13 5))))
    (:then_11
      (Default|SetRowTwelveFields _output_get (Class|VaRestJsonValue|AsString (Utilities|Array|Get(acopy) _returnvalue_14 1)) (Class|VaRestJsonValue|AsString (Utilities|Array|Get(acopy) _returnvalue_14 2)) (Class|VaRestJsonValue|AsString (Utilities|Array|Get(acopy) _returnvalue_14 3)) (Class|VaRestJsonValue|AsString (Utilities|Array|Get(acopy) _returnvalue_14 4)) (Class|VaRestJsonValue|AsString (Utilities|Array|Get(acopy) _returnvalue_14 5))))))

(event EventBeginPlay
  (bind _returnvalue (Class|VaRestSubsystem|ConstructVaRestRequestExt (|VaRestSubsystem) "GET" "x_www_form_urlencoded_url"))
  (bind _output_get (Variables|Default|SetRequest _returnvalue))
  (Class|VaRestRequestJSON|SetURL _output_get (Variables|Default|GetURL))
  (EventDispatchers|BindEventtoOnRequestComplete (Variables|Default|GetRequest) (delegate Custom|Success))
  (EventDispatchers|BindEventtoOnRequestFail (Variables|Default|GetRequest) (delegate Custom|Fail))
  (Class|VaRestRequestJSON|ExecuteProcessRequest (Variables|Default|GetRequest)))

(fn ConstructionScript)