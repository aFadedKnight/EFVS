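; Countdown Blueprint that animates five text actors, Text5 down to Text1, one after another when StartCountdown fires.
; Five chained timelines each lerp one actor between shared points A and B using a LogoMove track.
; As each timeline finishes, the next starts immediately via a Sequence, while the finished actor waits half a second before jumping to the world origin.
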(event Custom|Start%20Countdown
  (bind _text_5 (Variables|Default|GetText_5))
  (bind _text_4 (Variables|Default|GetText_4))
  (bind _text_3 (Variables|Default|GetText_3))
  (bind _text_2 (Variables|Default|GetText_2))
  (bind _text_1 (Variables|Default|GetText_1))
  (bind _logomove (Timeline|Timeline_0 PlayFromStart)
    (:Update
      (Transformation|SetActorLocation _text_5 (Math|Vector|Lerp(Vector) (Variables|Default|GetA) (Variables|Default|GetB) _logomove) false false))
    (:Finished
      (Utilities|FlowControl|Sequence
        (:then_0
          (Utilities|FlowControl|Delay 0.5)
          (Transformation|SetActorLocation _text_5 "0, 0, 0" false false))
        (:then_1
          (bind _logomove_2 (Timeline|Timeline_1 PlayFromStart)
            (:Update
              (Transformation|SetActorLocation _text_4 (Math|Vector|Lerp(Vector) (Variables|Default|GetA) (Variables|Default|GetB) _logomove_2) false false))
            (:Finished
              (Utilities|FlowControl|Sequence
                (:then_0
                  (Utilities|FlowControl|Delay 0.5)
                  (Transformation|SetActorLocation _text_4 "0, 0, 0" false false))
                (:then_1
                  (bind _logomove_3 (Timeline|Timeline_3 PlayFromStart)
                    (:Update
                      (Transformation|SetActorLocation _text_3 (Math|Vector|Lerp(Vector) (Variables|Default|GetA) (Variables|Default|GetB) _logomove_3) false false))
                    (:Finished
                      (Utilities|FlowControl|Sequence
                        (:then_0
                          (Utilities|FlowControl|Delay 0.5)
                          (Transformation|SetActorLocation _text_3 "0, 0, 0" false false))
                        (:then_1
                          (bind _logomove_4 (Timeline|Timeline_2 PlayFromStart)
                            (:Update
                              (Transformation|SetActorLocation _text_2 (Math|Vector|Lerp(Vector) (Variables|Default|GetA) (Variables|Default|GetB) _logomove_4) false false))
                            (:Finished
                              (Utilities|FlowControl|Sequence
                                (:then_0
                                  (Utilities|FlowControl|Delay 0.5)
                                  (Transformation|SetActorLocation _text_2 "0, 0, 0" false false))
                                (:then_1
                                  (bind _logomove_5 (Timeline|Timeline_4 PlayFromStart)
                                    (:Update
                                      (Transformation|SetActorLocation _text_1 (Math|Vector|Lerp(Vector) (Variables|Default|GetA) (Variables|Default|GetB) _logomove_5) false false))
                                    (:Finished
                                      (Utilities|FlowControl|Delay 0.5)
                                      (Transformation|SetActorLocation _text_1 "0, 0, 0" false false))))))))))))))))))))

(fn ConstructionScript)