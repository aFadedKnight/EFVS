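; BP_Logo is a logo actor that slides between two stored positions and swings its rotation.
; MoveUp and MoveDown drive separate timelines that lerp the location between End and End2.
; MoveDown enables the RotateLogo swing between two fixed angles.
; MoveUp clears the rotate flags, so the swing stops once it nears the Front rotation, settling the logo rather than snapping it.
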(event Custom|Rotator
  (if (Variables|Default|GetRotate)
    (Variables|Default|SetMoving true)
    (bind _rotate_amount (Timeline|RotateLogo PlayFromStart)
      (:Update
        (if (Variables|Default|GetMoving)
          _
          (elif (Math|Rotator|Equal(Rotator) (Variables|Default|GetFront) (Math|Rotator|Lerp(Rotator) "0,-30.000000, 0" "0,30.000000, 0" _rotate_amount) _rotate_amount)
            (CallFunction|Stop)))
        (Transformation|SetActorRotation (Math|Rotator|Lerp(Rotator) "0,-30.000000, 0" "0,30.000000, 0" _rotate_amount))))
    (else
      (Variables|Default|SetMoving false))))

(event Custom|Stop
  (bind _rotate_amount (Timeline|RotateLogo Stop)
    (:Update
      (if (Variables|Default|GetMoving)
        _
        (elif (Math|Rotator|Equal(Rotator) (Variables|Default|GetFront) (Math|Rotator|Lerp(Rotator) "0,-30.000000, 0" "0,30.000000, 0" _rotate_amount) _rotate_amount)
          (CallFunction|Stop)))
      (Transformation|SetActorRotation (Math|Rotator|Lerp(Rotator) "0,-30.000000, 0" "0,30.000000, 0" _rotate_amount)))))

(event Custom|MoveDown
  (Variables|Default|SetRotate true)
  (CallFunction|Rotator)
  (bind _output_get (Variables|Default|SetStart (Variables|Default|GetEnd)))
  (bind _output_get_2 (Variables|Default|SetEnd_2 (Variables|Default|GetEnd_2)))
  (bind _logomove (Timeline|Timeline_1 Play)
    (:Update
      (Transformation|SetActorLocation (Math|Vector|Lerp(Vector) _output_get _output_get_2 _logomove) false false))))

(event Custom|MoveUp
  (bind _output_get (Variables|Default|SetStart (Variables|Default|GetEnd_2)))
  (bind _output_get_2 (Variables|Default|SetEnd (Variables|Default|GetEnd)))
  (Utilities|FlowControl|Sequence
    (:then_0
      (bind _logomove (Timeline|Timeline_0 PlayFromStart)
        (:Update
          (Transformation|SetActorLocation (Math|Vector|Lerp(Vector) _output_get _output_get_2 _logomove) false false)
          (Variables|Default|SetRotate false)
          (CallFunction|Rotator))))))

(event EventBeginPlay
  (Input|EnableInput (Game|GetPlayerController 0))
  (CallFunction|Rotator))

(event Collision|EventActorBeginOverlap
  (params (OtherActor :type Actor%20Object%20Reference)))

(fn ConstructionScript)