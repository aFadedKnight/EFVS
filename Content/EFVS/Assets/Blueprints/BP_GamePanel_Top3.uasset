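; BP_GamePanel_Top3 is a panel actor that displays the first, second and third place teams for games.
; On BeginPlay it applies the Controller's games material to the talent panel mesh and fills three text components from the Controller's placement values.
; The construction script also sets the texts, using the Controller's game-one first place for both first and second, and not reading the Controller for third.
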(event EventBeginPlay
  (bind _controller (Variables|Default|GetController))
  (bind _output (Utilities|ResolveSoftReference _controller))
  (Rendering|Material|SetMaterial (Variables|Default|GetSM_TalentPanel) 2 (Variables|/Game/EFVS/Studio/Control/BP_Controller.BP_Controller_C|GetGamesMaterial _output))
  (Rendering|Components|TextRender|SetText (Variables|Default|GetFirstPlaceTeam) (Variables|/Game/EFVS/Studio/Control/BP_Controller.BP_Controller_C|GetFirst%20Place _output))
  (Rendering|Components|TextRender|SetText (Variables|Default|GetSecondPlaceTeam) (Variables|/Game/EFVS/Studio/Control/BP_Controller.BP_Controller_C|GetSecond%20Place _output))
  (Rendering|Components|TextRender|SetText (Variables|Default|GetThirdPlaceTeam) (Variables|/Game/EFVS/Studio/Control/BP_Controller.BP_Controller_C|GetThird%20Place _output)))

(event Collision|EventActorBeginOverlap
  (params (OtherActor :type Actor%20Object%20Reference)))

(event EventTick
  (params (DeltaSeconds :type Float%20%28single-precision%29)))

(fn ConstructionScript
  (bind _controller (Variables|Default|GetController))
  (bind _output (Utilities|ResolveSoftReference _controller))
  (bind _first_place_g1 (Variables|/Game/EFVS/Studio/Control/BP_Controller.BP_Controller_C|GetFirst%20Place%20G1 _output))
  (Rendering|Components|TextRender|SetText (Variables|Default|GetFirstPlaceTeam) _first_place_g1)
  (Rendering|Components|TextRender|SetText (Variables|Default|GetSecondPlaceTeam) _first_place_g1)
  (Rendering|Components|TextRender|SetText (Variables|Default|GetThirdPlaceTeam) (Variables|Default|GetThird%20Place%20Team)))