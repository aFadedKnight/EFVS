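; Studio A controller that themes the virtual set and moves the camera between Door, Hosts, Casters and TV views.
; Construction and BeginPlay look up the selected theme's DataTable row, setting material collection colors and monitor and host panel materials.
; To_ events choose a Level Sequence from the tracked CameraLocation, ignoring requests while one plays.
; An OSC server, created by a separate event, maps message addresses to those camera moves.
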(event Custom|OnMessage
  (params (Message :type OSC%20Message%20Structure%20%28by%20ref%29) (IPAddress :type String) (Port :type Integer))
  ;[1 1 1] OSC
  (Development|PrintString "Message Receiverd")
  (bind _returnvalue (Class|OSCManager|GetOSCMessageAddress Message))
  (bind _returnvalue_2 (Class|OSCManager|GetOSCAddressFullPath _returnvalue))
  (switch string _returnvalue_2
    (:/unreal/casters
      ;[0 0 0] Trigger camera to go to the casters
      (Utilities|IsValid (Variables|Default|GetLevelSequencePlayer)
        (:Is%20Valid
          (if (not (Audio|Components|Audio|IsPlaying (Variables|Default|GetLevelSequencePlayer)))
            (switch string (Variables|Default|GetCameraLocation) :!label _label
              (:Hosts
                (CallFunction|HoststoCasters))
              (:TV
                (CallFunction|TVtoCasters))
              (:Door
                (CallFunction|DoortoCasters)))
            (Variables|Default|SetCameraLocation "Casters")))
        (:Is%20Not%20Valid
          (goto _label))))
    (:/unreal/hosts
      ;[0 0 0] Trigger camera to go to the hosts
      (Utilities|IsValid (Variables|Default|GetLevelSequencePlayer)
        (:Is%20Valid
          (if (not (Audio|Components|Audio|IsPlaying (Variables|Default|GetLevelSequencePlayer)))
            (switch string (Variables|Default|GetCameraLocation) :!label _label_2
              (:Casters
                (CallFunction|CasterstoHost))
              (:TV
                (CallFunction|TVtoHost))
              (:Door
                (CallFunction|DoortoHost)))
            (Variables|Default|SetCameraLocation "Hosts")))
        (:Is%20Not%20Valid
          (goto _label_2))))
    (:/unreal/door
      ;[0 0 0] Trigger camera to go to the door
      (Utilities|IsValid (Variables|Default|GetLevelSequencePlayer)
        (:Is%20Valid
          (if (not (Audio|Components|Audio|IsPlaying (Variables|Default|GetLevelSequencePlayer)))
            (switch string (Variables|Default|GetCameraLocation) :!label _label_3
              (:Hosts
                (CallFunction|HoststoDoor))
              (:Casters
                (CallFunction|CasterstoDoor))
              (:TV
                (CallFunction|TVtoDoor)))
            (Variables|Default|SetCameraLocation "Door")))
        (:Is%20Not%20Valid
          (goto _label_3))))
    (:/unreal/tv
      ;[0 0 0] Trigger camera to go to the TV
      (Utilities|IsValid (Variables|Default|GetLevelSequencePlayer)
        (:Is%20Valid
          (if (not (Audio|Components|Audio|IsPlaying (Variables|Default|GetLevelSequencePlayer)))
            (switch string (Variables|Default|GetCameraLocation) :!label _label_4
              (:Hosts
                (CallFunction|HoststoTV))
              (:Casters
                (CallFunction|CasterstoTV))
              (:Door
                (CallFunction|DoortoTV)))
            (Variables|Default|SetCameraLocation "TV")))
        (:Is%20Not%20Valid
          (goto _label_4))))))

(event Custom|Door_To_Host
  ;[0 0 0] "Door to X" function definitions
  (bind (_outactor _returnvalue) (Sequencer|Player|CreateLevelSequencePlayer "/Game/EFVS/Studio/LevelSequences/CameraMoves/StudioA/LS_DoorToHost.LS_DoorToHost"))
  (Sequencer|Player|Play (Variables|/Script/LevelSequence.LevelSequenceActor|GetSequencePlayer _outactor) :!class /Script/MovieScene.MovieSceneSequencePlayer)
  (Variables|Default|SetLevelSequencePlayer _returnvalue))

(event Custom|TV_To_Casters
  ;[0 0 0] "TV to X" function definitions
  (bind (_outactor _returnvalue) (Sequencer|Player|CreateLevelSequencePlayer "/Game/EFVS/Studio/LevelSequences/CameraMoves/StudioA/LS_TVToCasters.LS_TVToCasters"))
  (Sequencer|Player|Play (Variables|/Script/LevelSequence.LevelSequenceActor|GetSequencePlayer _outactor) :!class /Script/MovieScene.MovieSceneSequencePlayer)
  (Variables|Default|SetLevelSequencePlayer _returnvalue))

(event Custom|Hosts_To_Door
  ;[0 0 0] "Hosts to X" function definitions
  (bind (_outactor _returnvalue) (Sequencer|Player|CreateLevelSequencePlayer "/Game/EFVS/Studio/LevelSequences/CameraMoves/StudioA/LS_HostToDoor.LS_HostToDoor"))
  (Sequencer|Player|Play (Variables|/Script/LevelSequence.LevelSequenceActor|GetSequencePlayer _outactor) :!class /Script/MovieScene.MovieSceneSequencePlayer)
  (Variables|Default|SetLevelSequencePlayer _returnvalue))

(event Custom|Door_To_Casters
  ;[0 0 0] "Door to X" function definitions
  (bind (_outactor _returnvalue) (Sequencer|Player|CreateLevelSequencePlayer "/Game/EFVS/Studio/LevelSequences/CameraMoves/StudioA/LS_DoorToCasters.LS_DoorToCasters"))
  (Sequencer|Player|Play (Variables|/Script/LevelSequence.LevelSequenceActor|GetSequencePlayer _outactor) :!class /Script/MovieScene.MovieSceneSequencePlayer)
  (Variables|Default|SetLevelSequencePlayer _returnvalue))

(event Custom|GetData
  (bind _returnvalue (Utilities|GetDataTableRow "/Game/EFVS/Studio/Customize/Themes/DT_Themes_StudioA.DT_Themes_StudioA" (Variables|Theme|GetTheme%20Select))
    (:then
      (Variables|Colors|SetColor_1_Selection (.color_01 _returnvalue))
      (Variables|Colors|SetColor_2_Selection (.color_02 _returnvalue))
      (Variables|Monitors|SetOut%20Row%20Monitor%20Front (.monitor_front _returnvalue))
      (Variables|Monitors|SetOut%20Row%20Monitor%20Back (.monitor_back _returnvalue))
      (Variables|Monitors|SetOut%20Row%20Monitor%20Side (.monitor_side _returnvalue))
      (Variables|Panels|SetOut%20Row%20Host%201 (.host_panel_1 _returnvalue))
      (Variables|Panels|SetOut%20Row%20Host%202 (.host_panel_2 _returnvalue))
      (Variables|Panels|SetOut%20Row%20Host%203 (.host_panel_3 _returnvalue))
      (Variables|Panels|SetOut%20Row%20Host%204 (.host_panel_4 _returnvalue))
      (Variables|Panels|SetOut%20Row%20Host%205 (.host_panel_5 _returnvalue)))))

(event Custom|SetCode
  (Variables|Theme|SetTheme%20Select (Utilities|String|StringToName (Utilities|String|EnumtoString (Variables|Theme|GetThemeSelect)))))

(event Custom|ApplyData
  (Utilities|FlowControl|Sequence
    (:then_0
      (Rendering|Material|SetVectorParameterValue "/Game/EFVS/Studio/Customize/MPC_Colors_StudioA.MPC_Colors_StudioA" "Color1" (Variables|Colors|GetColor_1_Selection) :!class /Script/Engine.KismetMaterialLibrary)
      (Rendering|Material|SetVectorParameterValue "/Game/EFVS/Studio/Customize/MPC_Colors_StudioA.MPC_Colors_StudioA" "Color2" (Variables|Colors|GetColor_2_Selection) :!class /Script/Engine.KismetMaterialLibrary))
    (:then_1
      (Rendering|Material|SetMaterial (Variables|/Script/Engine.StaticMeshActor|GetStaticMeshComponent (Variables|Monitors|GetMonitor_Front)) 0 (Variables|Monitors|GetOut%20Row%20Monitor%20Front)))
    (:then_2
      (Rendering|Material|SetMaterial (Variables|/Script/Engine.StaticMeshActor|GetStaticMeshComponent (Variables|Monitors|GetMonitor_Back)) 0 (Variables|Monitors|GetOut%20Row%20Monitor%20Back))
      (Variables|Default|SetBlackGlossy 0))
    (:then_3
      (Rendering|Material|SetMaterial (Variables|/Script/Engine.StaticMeshActor|GetStaticMeshComponent (Variables|Monitors|GetMonitor_Side)) 0 (Variables|Monitors|GetOut%20Row%20Monitor%20Side)))
    (:then_4
      (Rendering|Material|SetMaterial (Variables|/Script/Engine.StaticMeshActor|GetStaticMeshComponent (Variables|Panels|GetHost%201)) 1 (Variables|Panels|GetOut%20Row%20Host%201)))
    (:then_5
      (Rendering|Material|SetMaterial (Variables|/Script/Engine.StaticMeshActor|GetStaticMeshComponent (Variables|Panels|GetHost%202)) 1 (Variables|Panels|GetOut%20Row%20Host%202)))
    (:then_6
      (Rendering|Material|SetMaterial (Variables|/Script/Engine.StaticMeshActor|GetStaticMeshComponent (Variables|Panels|GetHost%203)) 1 (Variables|Panels|GetOut%20Row%20Host%203)))
    (:then_7
      (Rendering|Material|SetMaterial (Variables|/Script/Engine.StaticMeshActor|GetStaticMeshComponent (Variables|Panels|GetHost%204)) 1 (Variables|Panels|GetOut%20Row%20Host%204)))
    (:then_8
      (Rendering|Material|SetMaterial (Variables|/Script/Engine.StaticMeshActor|GetStaticMeshComponent (Variables|Panels|GetHost%205)) 1 (Variables|Panels|GetOut%20Row%20Host%205)))))

(event Custom|Casters_To_Host
  ;[0 0 0] "Casters to X" function definitions
  (bind (_outactor _returnvalue) (Sequencer|Player|CreateLevelSequencePlayer "/Game/EFVS/Studio/LevelSequences/CameraMoves/StudioA/LS_CastersToHost.LS_CastersToHost"))
  (Sequencer|Player|Play (Variables|/Script/LevelSequence.LevelSequenceActor|GetSequencePlayer _outactor) :!class /Script/MovieScene.MovieSceneSequencePlayer)
  (Variables|Default|SetLevelSequencePlayer _returnvalue))

(event Custom|To_Hosts
  ;[0 0 0] Trigger camera to go to the hosts
  (Utilities|IsValid (Variables|Default|GetLevelSequencePlayer)
    (:Is%20Valid
      (if (not (Audio|Components|Audio|IsPlaying (Variables|Default|GetLevelSequencePlayer)))
        (switch string (Variables|Default|GetCameraLocation) :!label _label
          (:Casters
            (CallFunction|CasterstoHost))
          (:TV
            (CallFunction|TVtoHost))
          (:Door
            (CallFunction|DoortoHost)))
        (Variables|Default|SetCameraLocation "Hosts")))
    (:Is%20Not%20Valid
      (goto _label))))

(event Custom|To_Casters
  ;[0 0 0] Trigger camera to go to the casters
  (Utilities|IsValid (Variables|Default|GetLevelSequencePlayer)
    (:Is%20Valid
      (if (not (Audio|Components|Audio|IsPlaying (Variables|Default|GetLevelSequencePlayer)))
        (switch string (Variables|Default|GetCameraLocation) :!label _label
          (:Hosts
            (CallFunction|HoststoCasters))
          (:TV
            (CallFunction|TVtoCasters))
          (:Door
            (CallFunction|DoortoCasters)))
        (Variables|Default|SetCameraLocation "Casters")))
    (:Is%20Not%20Valid
      (goto _label))))

(event Custom|To_Door
  ;[0 0 0] Trigger camera to go to the door
  (Utilities|IsValid (Variables|Default|GetLevelSequencePlayer)
    (:Is%20Valid
      (if (not (Audio|Components|Audio|IsPlaying (Variables|Default|GetLevelSequencePlayer)))
        (switch string (Variables|Default|GetCameraLocation) :!label _label
          (:Hosts
            (CallFunction|HoststoDoor))
          (:Casters
            (CallFunction|CasterstoDoor))
          (:TV
            (CallFunction|TVtoDoor)))
        (Variables|Default|SetCameraLocation "Door")))
    (:Is%20Not%20Valid
      (goto _label))))

(event Custom|To_TV
  ;[0 0 0] Trigger camera to go to the TV
  (Utilities|IsValid (Variables|Default|GetLevelSequencePlayer)
    (:Is%20Valid
      (if (not (Audio|Components|Audio|IsPlaying (Variables|Default|GetLevelSequencePlayer)))
        (switch string (Variables|Default|GetCameraLocation) :!label _label
          (:Hosts
            (CallFunction|HoststoTV))
          (:Casters
            (CallFunction|CasterstoTV))
          (:Door
            (CallFunction|DoortoTV)))
        (Variables|Default|SetCameraLocation "TV")))
    (:Is%20Not%20Valid
      (goto _label))))

(event Custom|TV_To_Host
  ;[0 0 0] "TV to X" function definitions
  (bind (_outactor _returnvalue) (Sequencer|Player|CreateLevelSequencePlayer "/Game/EFVS/Studio/LevelSequences/CameraMoves/StudioA/LS_TVToHost.LS_TVToHost"))
  (Sequencer|Player|Play (Variables|/Script/LevelSequence.LevelSequenceActor|GetSequencePlayer _outactor) :!class /Script/MovieScene.MovieSceneSequencePlayer)
  (Variables|Default|SetLevelSequencePlayer _returnvalue))

(event Custom|Casters_To_Door
  ;[0 0 0] "Casters to X" function definitions
  (bind (_outactor _returnvalue) (Sequencer|Player|CreateLevelSequencePlayer "/Game/EFVS/Studio/LevelSequences/CameraMoves/StudioA/LS_CastersToDoor.LS_CastersToDoor"))
  (Sequencer|Player|Play (Variables|/Script/LevelSequence.LevelSequenceActor|GetSequencePlayer _outactor) :!class /Script/MovieScene.MovieSceneSequencePlayer)
  (Variables|Default|SetLevelSequencePlayer _returnvalue))

(event Custom|TV_To_Door
  ;[0 0 0] "TV to X" function definitions
  (bind (_outactor _returnvalue) (Sequencer|Player|CreateLevelSequencePlayer "/Game/EFVS/Studio/LevelSequences/CameraMoves/StudioA/LS_TVToDoor.LS_TVToDoor"))
  (Sequencer|Player|Play (Variables|/Script/LevelSequence.LevelSequenceActor|GetSequencePlayer _outactor) :!class /Script/MovieScene.MovieSceneSequencePlayer)
  (Variables|Default|SetLevelSequencePlayer _returnvalue))

(event Custom|Hosts_To_Casters
  ;[0 0 0] "Hosts to X" function definitions
  (bind (_outactor _returnvalue) (Sequencer|Player|CreateLevelSequencePlayer "/Game/EFVS/Studio/LevelSequences/CameraMoves/StudioA/LS_HostToCasters.LS_HostToCasters"))
  (Sequencer|Player|Play (Variables|/Script/LevelSequence.LevelSequenceActor|GetSequencePlayer _outactor) :!class /Script/MovieScene.MovieSceneSequencePlayer)
  (Variables|Default|SetLevelSequencePlayer _returnvalue))

(event Custom|Door_To_TV
  ;[0 0 0] "Door to X" function definitions
  (bind (_outactor _returnvalue) (Sequencer|Player|CreateLevelSequencePlayer "/Game/EFVS/Studio/LevelSequences/CameraMoves/StudioA/LS_DoorToTV.LS_DoorToTV"))
  (Sequencer|Player|Play (Variables|/Script/LevelSequence.LevelSequenceActor|GetSequencePlayer _outactor) :!class /Script/MovieScene.MovieSceneSequencePlayer)
  (Variables|Default|SetLevelSequencePlayer _returnvalue))

(event Custom|Hosts_To_TV
  ;[0 0 0] "Hosts to X" function definitions
  (bind (_outactor _returnvalue) (Sequencer|Player|CreateLevelSequencePlayer "/Game/EFVS/Studio/LevelSequences/CameraMoves/StudioA/LS_HostToTV.LS_HostToTV"))
  (Sequencer|Player|Play (Variables|/Script/LevelSequence.LevelSequenceActor|GetSequencePlayer _outactor) :!class /Script/MovieScene.MovieSceneSequencePlayer)
  (Variables|Default|SetLevelSequencePlayer _returnvalue))

(event Custom|Casters_To_TV
  ;[0 0 0] "Casters to X" function definitions
  (bind (_outactor _returnvalue) (Sequencer|Player|CreateLevelSequencePlayer "/Game/EFVS/Studio/LevelSequences/CameraMoves/StudioA/LS_CastersToTv.LS_CastersToTv"))
  (Sequencer|Player|Play (Variables|/Script/LevelSequence.LevelSequenceActor|GetSequencePlayer _outactor) :!class /Script/MovieScene.MovieSceneSequencePlayer)
  (Variables|Default|SetLevelSequencePlayer _returnvalue))

(event Custom|CreateOSCServer
  ;[1 1 1] OSC
  (bind _returnvalue (Class|OSCManager|CreateOSCServer "0.0.0.0" 8000 false true "" 0))
  (bind _output_get (Variables|Default|SetOSCServer _returnvalue))
  (EventDispatchers|UnbindallEventsfromOnOscBundleReceived _returnvalue)
  (EventDispatchers|BindEventtoOnOscMessageReceived _output_get (EventDispatchers|CreateEvent :!event Custom|OnMessage)))

(event EventBeginPlay
  (Utilities|FlowControl|Sequence
    (:then_0
      (CallFunction|SetCode))
    (:then_1
      (CallFunction|GetData)
      (CallFunction|ApplyData))
    (:then_2
      (Variables|Default|SetCameraLocation "Door"))))

(fn ConstructionScript
  (Utilities|FlowControl|Sequence
    (:then_0
      (CallFunction|SetCode))
    (:then_1
      (CallFunction|GetData)
      (CallFunction|ApplyData))))