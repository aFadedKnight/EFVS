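; BP_CameraController drives a studio camera around a logo, apparently for an NDI output.
; The CircleLogo timeline starts on BeginPlay, sets camera position and replays through CameraCircleIM while Track is true.
; Tick uses look-at rotation to aim at the logo while tracking, which EnableTracking switches on.
; DisableTracking stops the circle, lerps the camera to an End position, then clears Track.
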(event Custom|EnableTracking
  (Variables|Default|SetTrack true))

(event Custom|DisableTracking
  (Utilities|FlowControl|Sequence
    (:then_0
      (bind _position (Timeline|CircleLogo Stop)
        (:Update
          (Transformation|SetActorLocation (Variables|Default|GetCamera) _position false false))
        (:Finished
          (if (Variables|Default|GetTrack)
            (CallFunction|CameraCircleIM)))))
    (:then_1
      (bind _output_get (Variables|Default|SetStart (Transformation|GetActorLocation (Variables|Default|GetCamera))))
      (bind _output_get_2 (Variables|Default|SetEnd (Variables|Default|GetEnd)))
      (bind _logomove (Timeline|Timeline_0 PlayFromStart)
        (:Update
          (Transformation|SetActorLocation (Variables|Default|GetCamera) (Math|Vector|Lerp(Vector) _output_get _output_get_2 _logomove) false false))
        (:Finished
          (Variables|Default|SetTrack false))))))

(event Custom|CameraCircleIM
  (bind _position (Timeline|CircleLogo PlayFromStart)
    (:Update
      (Transformation|SetActorLocation (Variables|Default|GetCamera) _position false false))
    (:Finished
      (if (Variables|Default|GetTrack)
        (CallFunction|CameraCircleIM)))))

(event EventBeginPlay
  (bind _position (Timeline|CircleLogo PlayFromStart)
    (:Update
      (Transformation|SetActorLocation (Variables|Default|GetCamera) _position false false))
    (:Finished
      (if (Variables|Default|GetTrack)
        (CallFunction|CameraCircleIM)))))

(event EventTick
  (params (DeltaSeconds :type Float%20%28single-precision%29))
  (bind _camera (Variables|Default|GetCamera))
  (if (Variables|Default|GetTrack)
    (Transformation|SetActorRotation _camera (Math|Rotator|FindLookatRotation (Transformation|GetActorLocation _camera) (Transformation|GetActorLocation (Variables|Default|GetLogo))))))

(fn ConstructionScript)