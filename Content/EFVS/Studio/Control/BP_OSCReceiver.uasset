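; BP_OSCReceiver lets external OSC messages remotely trigger studio control actions.
; On BeginPlay it creates a listening OSC server on a fixed port and binds a handler for received messages.
; The handler switches on each message's address path and calls the matching Controller function, such as Casters, Countdown, Door, ToggleLeaderboard or Update.
; Only the address selects the action; message arguments are not read.
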(event Custom|OnMessage
  (params (Message :type OSC%20Message%20Structure%20%28by%20ref%29) (IPAddress :type String) (Port :type Integer))
  (bind _controller (Variables|Default|GetController))
  (bind _output (Utilities|ResolveSoftReference _controller))
  (Development|PrintString "Message Receiverd")
  (bind _returnvalue (Class|OSCManager|GetOSCMessageAddress Message))
  (bind _returnvalue_2 (Class|OSCManager|GetOSCAddressFullPath _returnvalue))
  (switch string _returnvalue_2
    (:/osc/casters
      (Default|Casters _output))
    (:/osc/countdown
      (Default|Countdown _output))
    (:/osc/default
      (Default|Default _output))
    (:/osc/door
      (Default|Door _output))
    (:/osc/hosts
      (Default|Hosts _output))
    (:/osc/recap
      (Default|Recap _output))
    (:/osc/togglelb
      (Default|ToggleLeaderboard _output))
    (:/osc/update
      (Default|Update _output))))

(event EventBeginPlay
  (bind _returnvalue (Class|OSCManager|CreateOSCServer "0.0.0.0" 8000 false true "" 0))
  (bind _output_get (Variables|Default|SetOSCServer _returnvalue))
  (EventDispatchers|UnbindallEventsfromOnOscBundleReceived _returnvalue)
  (EventDispatchers|BindEventtoOnOscMessageReceived _output_get (EventDispatchers|CreateEvent :!event Custom|OnMessage)))

(fn ConstructionScript)