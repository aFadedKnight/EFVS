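; Studio controller for a broadcast set that moves the camera between Default, Hosts, Casters, Recap and Door views.
; Each switch plays a level sequence for that transition, guarded against overlaps; Default hands back to the tracking camera controller.
; A theme data table row sets logo, screen and panel materials, collection colors and lights.
; It also rebuilds one to seven top-three game panels and triggers the leaderboard and countdown.
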(event Custom|HostsToDoor
  ;[0 0 0] "Hosts to X" function definitions
  (bind (_outactor _returnvalue) (Sequencer|Player|CreateLevelSequencePlayer "/Game/EFVS/Studio/LevelSequences/CameraMoves/StudioB/LS_HostToDoor.LS_HostToDoor"))
  (Sequencer|Player|Play (Variables|/Script/LevelSequence.LevelSequenceActor|GetSequencePlayer _outactor) :!class /Script/MovieScene.MovieSceneSequencePlayer)
  (Variables|Default|SetActive_Sequence _returnvalue))

(event Custom|Countdown
  (if (Utilities|Enum|Equal(Enum) (Variables|Default|GetLocations) "NewEnumerator0")
    (Default|StartCountdown (Utilities|ResolveSoftReference (Variables|Blueprints|GetCountdownBP)))))

(event Custom|RecapToCasters
  ;[0 0 0] "Recap to X" function definitions
  (bind (_outactor _returnvalue) (Sequencer|Player|CreateLevelSequencePlayer "/Game/EFVS/Studio/LevelSequences/CameraMoves/StudioB/LS_RecapToCasters.LS_RecapToCasters"))
  (Sequencer|Player|Play (Variables|/Script/LevelSequence.LevelSequenceActor|GetSequencePlayer _outactor) :!class /Script/MovieScene.MovieSceneSequencePlayer)
  (Variables|Default|SetActive_Sequence _returnvalue))

(event Custom|Toggle%20Leaderboard
  (if (Utilities|Enum|Equal(Enum) (Variables|Default|GetLocations) "NewEnumerator1")
    (Default|ToggleLeaderboard (Utilities|ResolveSoftReference (Variables|Blueprints|GetLeaderboard)))))

(event Custom|DoorToCasters
  ;[0 0 0] "Door to X" function definitions
  (bind (_outactor _returnvalue) (Sequencer|Player|CreateLevelSequencePlayer "/Game/EFVS/Studio/LevelSequences/CameraMoves/StudioB/LS_DoorToDefault.LS_DoorToDefault"))
  (Sequencer|Player|Play (Variables|/Script/LevelSequence.LevelSequenceActor|GetSequencePlayer _outactor) :!class /Script/MovieScene.MovieSceneSequencePlayer)
  (Variables|Default|SetActive_Sequence _returnvalue))

(event Custom|Update
  (Utilities|FlowControl|Sequence
    (:then_0
      (Utilities|Array|Clear (Variables|GamePlacements|GetFirst%20Place%20Array))
      (Utilities|Array|Add (Variables|GamePlacements|GetFirst%20Place%20Array) (Variables|GamePlacements|GetFirst%20Place%20G1))
      (Utilities|Array|Add (Variables|GamePlacements|GetFirst%20Place%20Array) (Variables|GamePlacements|GetFirst%20Place%20G2))
      (Utilities|Array|Add (Variables|GamePlacements|GetFirst%20Place%20Array) (Variables|GamePlacements|GetFirst%20Place%20G3))
      (Utilities|Array|Add (Variables|GamePlacements|GetFirst%20Place%20Array) (Variables|GamePlacements|GetFirst%20Place%20G4))
      (Utilities|Array|Add (Variables|GamePlacements|GetFirst%20Place%20Array) (Variables|GamePlacements|GetFirst%20Place%20G5))
      (Utilities|Array|Add (Variables|GamePlacements|GetFirst%20Place%20Array) (Variables|GamePlacements|GetFirst%20Place%20G6))
      (Utilities|Array|Add (Variables|GamePlacements|GetFirst%20Place%20Array) (Variables|GamePlacements|GetFirst%20Place%20G7)))
    (:then_1
      (Utilities|Array|Clear (Variables|GamePlacements|GetSecond%20Place%20Array))
      (Utilities|Array|Add (Variables|GamePlacements|GetSecond%20Place%20Array) (Variables|GamePlacements|GetSecond%20Place%20G1))
      (Utilities|Array|Add (Variables|GamePlacements|GetSecond%20Place%20Array) (Variables|GamePlacements|GetSecond%20Place%20G2))
      (Utilities|Array|Add (Variables|GamePlacements|GetSecond%20Place%20Array) (Variables|GamePlacements|GetSecond%20Place%20G3))
      (Utilities|Array|Add (Variables|GamePlacements|GetSecond%20Place%20Array) (Variables|GamePlacements|GetSecond%20Place%20G4))
      (Utilities|Array|Add (Variables|GamePlacements|GetSecond%20Place%20Array) (Variables|GamePlacements|GetSecond%20Place%20G5))
      (Utilities|Array|Add (Variables|GamePlacements|GetSecond%20Place%20Array) (Variables|GamePlacements|GetSecond%20Place%20G6))
      (Utilities|Array|Add (Variables|GamePlacements|GetSecond%20Place%20Array) (Variables|GamePlacements|GetSecond%20Place%20G7)))
    (:then_2
      (Utilities|Array|Clear (Variables|GamePlacements|GetThird%20Place%20Array))
      (Utilities|Array|Add (Variables|GamePlacements|GetThird%20Place%20Array) (Variables|GamePlacements|GetThird%20Place%20G1))
      (Utilities|Array|Add (Variables|GamePlacements|GetThird%20Place%20Array) (Variables|GamePlacements|GetThird%20Place%20G2))
      (Utilities|Array|Add (Variables|GamePlacements|GetThird%20Place%20Array) (Variables|GamePlacements|GetThird%20Place%20G3))
      (Utilities|Array|Add (Variables|GamePlacements|GetThird%20Place%20Array) (Variables|GamePlacements|GetThird%20Place%20G4))
      (Utilities|Array|Add (Variables|GamePlacements|GetThird%20Place%20Array) (Variables|GamePlacements|GetThird%20Place%20G5))
      (Utilities|Array|Add (Variables|GamePlacements|GetThird%20Place%20Array) (Variables|GamePlacements|GetThird%20Place%20G6))
      (Utilities|Array|Add (Variables|GamePlacements|GetThird%20Place%20Array) (Variables|GamePlacements|GetThird%20Place%20G7)))
    (:then_3
      (CallFunction|SetCode))
    (:then_4
      (CallFunction|GetData)
      (CallFunction|ApplyData))
    (:then_6
      (Variables|Default|SetNumberofGames_Int (Math|Conversions|ToInteger(Byte) (Utilities|String|ToString(Text) (Variables|GamePlacements|GetNumberofGames))))
      (if (>= (Variables|Default|GetNumberofGames_Int) 8)
        (Variables|Default|SetNumberofGames_Int 7)
        (Variables|GamePlacements|SetNumberofGames (Utilities|Text|ToText(Integer) 0))
        (elif (<= (Variables|Default|GetNumberofGames_Int) 0)
          (bind _output_get (Variables|Default|SetNumberofGames_Int 1))
          (Variables|GamePlacements|SetNumberofGames (Utilities|Text|ToText(Integer) _output_get))))
      (for _array_element (Actor|GetAllChildActors (Utilities|ResolveSoftReference (Variables|Blueprints|GetGames)) true)
        (Utilities|IsValid _array_element
          (:Is%20Valid
            (Actor|DestroyActor _array_element))))
      (if (not (<= (- (Variables|Default|GetNumberofGames_Int) 1) -1))
        (Variables|Default|SetRelative%20Transform (Math|Transform|MakeTransform (Math|Vector|MakeVector (Math|Conversions|ToFloat(Integer) (- -85 (/ (* (Variables|Default|GetNumberofGames_Int) 170) 2))) 0.0 0.0) "0, 0, 0" "1,1,1"))
        (for _index (range 0 (- (Variables|Default|GetNumberofGames_Int) 1))
          (Utilities|FlowControl|Sequence
            (:then_0
              (Variables|GamePlacements|SetFirst%20Place (Utilities|Array|Get(acopy) (Variables|GamePlacements|GetFirst%20Place%20Array) _index)))
            (:then_1
              (Variables|GamePlacements|SetSecond%20Place (Utilities|Array|Get(acopy) (Variables|GamePlacements|GetSecond%20Place%20Array) _index)))
            (:then_2
              (Variables|GamePlacements|SetThird%20Place (Utilities|Array|Get(acopy) (Variables|GamePlacements|GetThird%20Place%20Array) _index)))
            (:then_3
              (Variables|Default|SetRelative%20Transform (Math|Transform|MakeTransform (Math|Vector|MakeVector (+ (.x (.location (Variables|Default|GetRelative%20Transform))) 1.7e+02) 0.0 0.0) "0, 0, 0" "1,1,1"))
              (bind _returnvalue (AddComponent|AddChildActorComponent (Utilities|ResolveSoftReference (Variables|Blueprints|GetGames)) false (Variables|Default|GetRelative%20Transform)))
              (ChildActorComponent|SetChildActorClass _returnvalue "/Game/EFVS/Assets/Blueprints/BP_GamePanel_Top3.BP_GamePanel_Top3_C"))))))))

(event Custom|DoorToHost
  ;[0 0 0] "Door to X" function definitions
  (bind (_outactor _returnvalue) (Sequencer|Player|CreateLevelSequencePlayer "/Game/EFVS/Studio/LevelSequences/CameraMoves/StudioB/LS_DoorToHost.LS_DoorToHost"))
  (Sequencer|Player|Play (Variables|/Script/LevelSequence.LevelSequenceActor|GetSequencePlayer _outactor) :!class /Script/MovieScene.MovieSceneSequencePlayer)
  (Variables|Default|SetActive_Sequence _returnvalue))

(event Custom|SetCode
  (Variables|Default|SetRow%20Name (Utilities|String|StringToName (Utilities|String|EnumtoString (Variables|Theme|GetThemeSelect)))))

(event Custom|DoorToRecap
  ;[0 0 0] "Door to X" function definitions
  (bind (_outactor _returnvalue) (Sequencer|Player|CreateLevelSequencePlayer "/Game/EFVS/Studio/LevelSequences/CameraMoves/StudioB/LS_DoorToRecap.LS_DoorToRecap"))
  (Sequencer|Player|Play (Variables|/Script/LevelSequence.LevelSequenceActor|GetSequencePlayer _outactor) :!class /Script/MovieScene.MovieSceneSequencePlayer)
  (Variables|Default|SetActive_Sequence _returnvalue))

(event Custom|DefaultToDoor
  ;[0 0 0] "Default to X" function definitions
  (Default|MoveUp (Utilities|ResolveSoftReference (Variables|Blueprints|GetLogo)))
  (Default|DisableTracking (Utilities|ResolveSoftReference (Variables|Blueprints|GetCameraController)))
  (Utilities|FlowControl|Delay 1.0)
  (bind _outactor (Sequencer|Player|CreateLevelSequencePlayer "/Game/EFVS/Studio/LevelSequences/CameraMoves/StudioB/LS_DefaultToDoor.LS_DefaultToDoor"))
  (Sequencer|Player|Play (Variables|/Script/LevelSequence.LevelSequenceActor|GetSequencePlayer _outactor) :!class /Script/MovieScene.MovieSceneSequencePlayer)
  (Variables|Default|SetActive_Sequence (Variables|/Script/LevelSequence.LevelSequenceActor|GetSequencePlayer _outactor))
  (Utilities|FlowControl|Delay 5.0)
  (Variables|Default|SetCamMoving false))

(event Custom|GetData
  (bind _returnvalue (Utilities|GetDataTableRow "/Game/EFVS/Assets/Themes/DT_Themes.DT_Themes" (Variables|Default|GetRow%20Name))
    (:then
      (Variables|Colors|SetColor_01_selection (.primarycolor _returnvalue))
      (Variables|Colors|SetColor_02_selection (.secondarycolor _returnvalue))
      (Components|StaticMesh|SetStaticMesh (Variables|/Game/EFVS/Assets/Blueprints/BP_Logo.BP_Logo_C|GetLogo (Variables|Blueprints|GetBP_Logo)) (.logomesh _returnvalue))
      (Rendering|Material|SetMaterial (Variables|/Script/Engine.StaticMeshActor|GetStaticMeshComponent (Variables|Meshes|GetCurvedMonitor)) 1 (.curvedscreen _returnvalue))
      (Variables|Default|SetGamesMaterial (.recapbackground _returnvalue))
      (|PanelMaterials (.hostpanel1 _returnvalue) (.hostpanel2 _returnvalue) (.hostpanel3 _returnvalue) (.casterpanel1 _returnvalue) (.casterpanel2 _returnvalue)))))

(event Custom|RecapToDefault
  (bind _cameracontroller (Variables|Blueprints|GetCameraController))
  (bind _output (Utilities|ResolveSoftReference _cameracontroller))
  ;[0 0 0] "Recap to X" function definitions
  (bind _outactor (Sequencer|Player|CreateLevelSequencePlayer "/Game/EFVS/Studio/LevelSequences/CameraMoves/StudioB/LS_RecapToDefault.LS_RecapToDefault"))
  (Sequencer|Player|Play (Variables|/Script/LevelSequence.LevelSequenceActor|GetSequencePlayer _outactor) :!class /Script/MovieScene.MovieSceneSequencePlayer)
  (Default|MoveDown (Utilities|ResolveSoftReference (Variables|Blueprints|GetLogo)))
  (Utilities|FlowControl|Delay 3.5)
  (Default|EnableTracking _output)
  (Utilities|FlowControl|Delay 0.6)
  (Default|CameraCircleIM _output)
  (Variables|Default|SetActive_Sequence (Variables|/Game/EFVS/Studio/NDI/Outputs/NDIOutput01/BP_CameraController.BP_CameraController_C|GetActive_Sequence (Utilities|ResolveSoftReference (Variables|Blueprints|GetCameraController)))))

(event Custom|DefaultToCasters
  ;[0 0 0] "Default to X" function definitions
  (Default|MoveUp (Utilities|ResolveSoftReference (Variables|Blueprints|GetLogo)))
  (Default|DisableTracking (Utilities|ResolveSoftReference (Variables|Blueprints|GetCameraController)))
  (Utilities|FlowControl|Delay 1.0)
  (bind _outactor (Sequencer|Player|CreateLevelSequencePlayer "/Game/EFVS/Studio/LevelSequences/CameraMoves/StudioB/LS_DefaultToCasters.LS_DefaultToCasters"))
  (Sequencer|Player|Play (Variables|/Script/LevelSequence.LevelSequenceActor|GetSequencePlayer _outactor) :!class /Script/MovieScene.MovieSceneSequencePlayer)
  (Variables|Default|SetActive_Sequence (Variables|/Script/LevelSequence.LevelSequenceActor|GetSequencePlayer _outactor))
  (Utilities|FlowControl|Delay 5.0)
  (Variables|Default|SetCamMoving false))

(event Custom|CastersToDefault
  (bind _cameracontroller (Variables|Blueprints|GetCameraController))
  (bind _output (Utilities|ResolveSoftReference _cameracontroller))
  ;[0 0 0] "Casters to X" function definitions
  (bind _outactor (Sequencer|Player|CreateLevelSequencePlayer "/Game/EFVS/Studio/LevelSequences/CameraMoves/StudioB/LS_CastersToDefault.LS_CastersToDefault"))
  (Sequencer|Player|Play (Variables|/Script/LevelSequence.LevelSequenceActor|GetSequencePlayer _outactor) :!class /Script/MovieScene.MovieSceneSequencePlayer)
  (Default|MoveDown (Utilities|ResolveSoftReference (Variables|Blueprints|GetLogo)))
  (Utilities|FlowControl|Delay 3.0)
  (Default|EnableTracking _output)
  (Utilities|FlowControl|Delay 0.6)
  (Default|CameraCircleIM _output)
  (Variables|Default|SetActive_Sequence (Variables|/Game/EFVS/Studio/NDI/Outputs/NDIOutput01/BP_CameraController.BP_CameraController_C|GetActive_Sequence (Utilities|ResolveSoftReference (Variables|Blueprints|GetCameraController)))))

(event Custom|ApplyData
  (bind _color_01_selection (Variables|Colors|GetColor_01_selection))
  (bind _color_02_selection (Variables|Colors|GetColor_02_selection))
  (Rendering|Material|SetVectorParameterValue "/Game/EFVS/Assets/Themes/MPC_Colors.MPC_Colors" "Color1" (Variables|Colors|GetColor_01_selection) :!class /Script/Engine.KismetMaterialLibrary)
  (Rendering|Material|SetVectorParameterValue "/Game/EFVS/Assets/Themes/MPC_Colors.MPC_Colors" "Color2" (Variables|Colors|GetColor_02_selection) :!class /Script/Engine.KismetMaterialLibrary)
  (Rendering|Components|Light|SetLightColor (Variables|/Script/Engine.PointLight|GetPointLightComponent (Variables|Lights|GetMiddleLight)) _color_01_selection true)
  (Rendering|Components|Light|SetLightColor (Variables|/Script/Engine.Light|GetLightComponent (Variables|Lights|GetBackRightLight)) _color_01_selection true)
  (Rendering|Components|Light|SetLightColor (Variables|/Script/Engine.Light|GetLightComponent (Variables|Lights|GetBackLeftLight)) _color_01_selection true)
  (Rendering|Components|Light|SetLightColor (Variables|/Script/Engine.Light|GetLightComponent (Variables|Lights|GetFrontRightLight)) _color_02_selection true)
  (Rendering|Components|Light|SetLightColor (Variables|/Script/Engine.Light|GetLightComponent (Variables|Lights|GetFrontLeftLight)) _color_02_selection true))

(event Custom|Hosts
  ;[0 0 0] Trigger camera to go to the hosts
  (Utilities|IsValid (Variables|Default|GetActive_Sequence)
    (:Is%20Valid
      (if (not (Variables|Default|GetCamMoving))
        (if (not (Audio|Components|Audio|IsPlaying (Variables|Default|GetActive_Sequence)))
          (switch Utilities|FlowControl|Switch|SwitchonEN_Locations (Variables|Default|GetLocations) :!label _label
            (:NewEnumerator0
              (CallFunction|DefaulttoHosts))
            (:NewEnumerator2
              (CallFunction|CasterstoHost))
            (:NewEnumerator7
              (CallFunction|RecaptoHost))
            (:NewEnumerator4
              (CallFunction|DoortoHost)))
          (Variables|Default|SetLocations "NewEnumerator1"))))
    (:Is%20Not%20Valid
      (goto _label))))

(event Custom|Door
  ;[0 0 0] Trigger camera to go to the door
  (Utilities|IsValid (Variables|Default|GetActive_Sequence)
    (:Is%20Valid
      (if (not (Variables|Default|GetCamMoving))
        (if (not (Audio|Components|Audio|IsPlaying (Variables|Default|GetActive_Sequence)))
          (switch Utilities|FlowControl|Switch|SwitchonEN_Locations (Variables|Default|GetLocations) :!label _label
            (:NewEnumerator0
              (CallFunction|DefaulttoDoor))
            (:NewEnumerator1
              (CallFunction|HoststoDoor))
            (:NewEnumerator2
              (CallFunction|CasterstoDoor))
            (:NewEnumerator7
              (CallFunction|RecaptoDoor)))
          (Variables|Default|SetLocations "NewEnumerator4"))))
    (:Is%20Not%20Valid
      (goto _label))))

(event Custom|Default
  ;[0 0 0] Trigger camera to go to Default
  (Utilities|IsValid (Variables|Default|GetActive_Sequence)
    (:Is%20Valid
      (if (not (Audio|Components|Audio|IsPlaying (Variables|Default|GetActive_Sequence)))
        (Variables|Default|SetCamMoving true)
        (switch Utilities|FlowControl|Switch|SwitchonEN_Locations (Variables|Default|GetLocations) :!label _label
          (:NewEnumerator1
            (CallFunction|HoststoDefault))
          (:NewEnumerator2
            (CallFunction|CasterstoDefault))
          (:NewEnumerator7
            (CallFunction|RecaptoDefault))
          (:NewEnumerator4
            (CallFunction|DoortoDefault)))
        (Variables|Default|SetLocations "NewEnumerator0")))
    (:Is%20Not%20Valid
      (goto _label))))

(event Custom|Recap
  ;[0 0 0] Trigger camera to go to the Recap
  (Utilities|IsValid (Variables|Default|GetActive_Sequence)
    (:Is%20Valid
      (if (not (Variables|Default|GetCamMoving))
        (if (not (Audio|Components|Audio|IsPlaying (Variables|Default|GetActive_Sequence)))
          (switch Utilities|FlowControl|Switch|SwitchonEN_Locations (Variables|Default|GetLocations) :!label _label
            (:NewEnumerator0
              (CallFunction|DefaulttoRecap))
            (:NewEnumerator1
              (CallFunction|HoststoRecap))
            (:NewEnumerator2
              (CallFunction|CasterstoRecap))
            (:NewEnumerator4
              (CallFunction|DoortoRecap)))
          (Variables|Default|SetLocations "NewEnumerator7"))))
    (:Is%20Not%20Valid
      (goto _label))))

(event Custom|CastersToHost
  ;[0 0 0] "Casters to X" function definitions
  (bind (_outactor _returnvalue) (Sequencer|Player|CreateLevelSequencePlayer "/Game/EFVS/Studio/LevelSequences/CameraMoves/StudioB/LS_CastersToHost.LS_CastersToHost"))
  (Sequencer|Player|Play (Variables|/Script/LevelSequence.LevelSequenceActor|GetSequencePlayer _outactor) :!class /Script/MovieScene.MovieSceneSequencePlayer)
  (Variables|Default|SetActive_Sequence _returnvalue))

(event Custom|RecapToHost
  ;[0 0 0] "Recap to X" function definitions
  (bind (_outactor _returnvalue) (Sequencer|Player|CreateLevelSequencePlayer "/Game/EFVS/Studio/LevelSequences/CameraMoves/StudioB/LS_RecapToHosts.LS_RecapToHosts"))
  (Sequencer|Player|Play (Variables|/Script/LevelSequence.LevelSequenceActor|GetSequencePlayer _outactor) :!class /Script/MovieScene.MovieSceneSequencePlayer)
  (Variables|Default|SetActive_Sequence _returnvalue))

(event Custom|CastersToDoor
  ;[0 0 0] "Casters to X" function definitions
  (bind (_outactor _returnvalue) (Sequencer|Player|CreateLevelSequencePlayer "/Game/EFVS/Studio/LevelSequences/CameraMoves/StudioB/LSCastersToDoor.LSCastersToDoor"))
  (Sequencer|Player|Play (Variables|/Script/LevelSequence.LevelSequenceActor|GetSequencePlayer _outactor) :!class /Script/MovieScene.MovieSceneSequencePlayer)
  (Variables|Default|SetActive_Sequence _returnvalue))

(event Custom|CastersToRecap
  ;[0 0 0] "Casters to X" function definitions
  (bind (_outactor _returnvalue) (Sequencer|Player|CreateLevelSequencePlayer "/Game/EFVS/Studio/LevelSequences/CameraMoves/StudioB/LS_CastersToRecap.LS_CastersToRecap"))
  (Sequencer|Player|Play (Variables|/Script/LevelSequence.LevelSequenceActor|GetSequencePlayer _outactor) :!class /Script/MovieScene.MovieSceneSequencePlayer)
  (Variables|Default|SetActive_Sequence _returnvalue))

(event Custom|HostsToCasters
  ;[0 0 0] "Hosts to X" function definitions
  (bind (_outactor _returnvalue) (Sequencer|Player|CreateLevelSequencePlayer "/Game/EFVS/Studio/LevelSequences/CameraMoves/StudioB/LS_HostToCasters.LS_HostToCasters"))
  (Sequencer|Player|Play (Variables|/Script/LevelSequence.LevelSequenceActor|GetSequencePlayer _outactor) :!class /Script/MovieScene.MovieSceneSequencePlayer)
  (Variables|Default|SetActive_Sequence _returnvalue))

(event Custom|Intermission%20to%20Host
  (Default|MoveUp (Utilities|ResolveSoftReference (Variables|Blueprints|GetLogo)))
  (Default|DisableTracking (Utilities|ResolveSoftReference (Variables|Blueprints|GetCameraController))))

(event Custom|Casters
  ;[0 0 0] Trigger camera to go to the casters
  (Utilities|IsValid (Variables|Default|GetActive_Sequence)
    (:Is%20Valid
      (if (not (Variables|Default|GetCamMoving))
        (if (not (Audio|Components|Audio|IsPlaying (Variables|Default|GetActive_Sequence)))
          (switch Utilities|FlowControl|Switch|SwitchonEN_Locations (Variables|Default|GetLocations) :!label _label
            (:NewEnumerator0
              (CallFunction|DefaulttoCasters))
            (:NewEnumerator1
              (CallFunction|HoststoCasters))
            (:NewEnumerator7
              (CallFunction|RecaptoCasters))
            (:NewEnumerator4
              (CallFunction|DoortoCasters)))
          (Variables|Default|SetLocations "NewEnumerator2"))))
    (:Is%20Not%20Valid
      (goto _label))))

(event Custom|DefaultToHosts
  ;[0 0 0] "Default to X" function definitions
  (Default|MoveUp (Utilities|ResolveSoftReference (Variables|Blueprints|GetLogo)))
  (Default|DisableTracking (Utilities|ResolveSoftReference (Variables|Blueprints|GetCameraController)))
  (Utilities|FlowControl|Delay 1.0)
  (bind _outactor (Sequencer|Player|CreateLevelSequencePlayer "/Game/EFVS/Studio/LevelSequences/CameraMoves/StudioB/LS_DefaultToHosts.LS_DefaultToHosts"))
  (Sequencer|Player|Play (Variables|/Script/LevelSequence.LevelSequenceActor|GetSequencePlayer _outactor) :!class /Script/MovieScene.MovieSceneSequencePlayer)
  (Variables|Default|SetActive_Sequence (Variables|/Script/LevelSequence.LevelSequenceActor|GetSequencePlayer _outactor))
  (Utilities|FlowControl|Delay 5.0)
  (Variables|Default|SetCamMoving false))

(event Custom|RecapToDoor
  ;[0 0 0] "Recap to X" function definitions
  (bind (_outactor _returnvalue) (Sequencer|Player|CreateLevelSequencePlayer "/Game/EFVS/Studio/LevelSequences/CameraMoves/StudioB/LS_RecapToDoor.LS_RecapToDoor"))
  (Sequencer|Player|Play (Variables|/Script/LevelSequence.LevelSequenceActor|GetSequencePlayer _outactor) :!class /Script/MovieScene.MovieSceneSequencePlayer)
  (Variables|Default|SetActive_Sequence _returnvalue))

(event Custom|HostsToRecap
  ;[0 0 0] "Hosts to X" function definitions
  (bind (_outactor _returnvalue) (Sequencer|Player|CreateLevelSequencePlayer "/Game/EFVS/Studio/LevelSequences/CameraMoves/StudioB/LS_HostToRecap.LS_HostToRecap"))
  (Sequencer|Player|Play (Variables|/Script/LevelSequence.LevelSequenceActor|GetSequencePlayer _outactor) :!class /Script/MovieScene.MovieSceneSequencePlayer)
  (Variables|Default|SetActive_Sequence _returnvalue))

(event Custom|DoorToDefault
  (bind _cameracontroller (Variables|Blueprints|GetCameraController))
  (bind _output (Utilities|ResolveSoftReference _cameracontroller))
  ;[0 0 0] "Door to X" function definitions
  (bind _outactor (Sequencer|Player|CreateLevelSequencePlayer "/Game/EFVS/Studio/LevelSequences/CameraMoves/StudioB/LS_DoorToDefault.LS_DoorToDefault"))
  (Sequencer|Player|Play (Variables|/Script/LevelSequence.LevelSequenceActor|GetSequencePlayer _outactor) :!class /Script/MovieScene.MovieSceneSequencePlayer)
  (Default|MoveDown (Utilities|ResolveSoftReference (Variables|Blueprints|GetLogo)))
  (Utilities|FlowControl|Delay 3.0)
  (Default|EnableTracking _output)
  (Utilities|FlowControl|Delay 0.6)
  (Default|CameraCircleIM _output)
  (Variables|Default|SetActive_Sequence (Variables|/Game/EFVS/Studio/NDI/Outputs/NDIOutput01/BP_CameraController.BP_CameraController_C|GetActive_Sequence (Utilities|ResolveSoftReference (Variables|Blueprints|GetCameraController)))))

(event Custom|HostsToDefault
  (bind _cameracontroller (Variables|Blueprints|GetCameraController))
  (bind _output (Utilities|ResolveSoftReference _cameracontroller))
  ;[0 0 0] "Hosts to X" function definitions
  (bind _outactor (Sequencer|Player|CreateLevelSequencePlayer "/Game/EFVS/Studio/LevelSequences/CameraMoves/StudioB/LS_HostToDefault.LS_HostToDefault"))
  (Sequencer|Player|Play (Variables|/Script/LevelSequence.LevelSequenceActor|GetSequencePlayer _outactor) :!class /Script/MovieScene.MovieSceneSequencePlayer)
  (Default|MoveDown (Utilities|ResolveSoftReference (Variables|Blueprints|GetLogo)))
  (Utilities|FlowControl|Delay 3.0)
  (Default|EnableTracking _output)
  (Utilities|FlowControl|Delay 0.5)
  (Default|CameraCircleIM _output)
  (Variables|Default|SetActive_Sequence (Variables|/Game/EFVS/Studio/NDI/Outputs/NDIOutput01/BP_CameraController.BP_CameraController_C|GetActive_Sequence (Utilities|ResolveSoftReference (Variables|Blueprints|GetCameraController)))))

(event Custom|DefaultToRecap
  ;[0 0 0] "Default to X" function definitions
  (Default|MoveUp (Utilities|ResolveSoftReference (Variables|Blueprints|GetLogo)))
  (Default|DisableTracking (Utilities|ResolveSoftReference (Variables|Blueprints|GetCameraController)))
  (Utilities|FlowControl|Delay 1.0)
  (bind _outactor (Sequencer|Player|CreateLevelSequencePlayer "/Game/EFVS/Studio/LevelSequences/CameraMoves/StudioB/LS_DefaultToRecap.LS_DefaultToRecap"))
  (Sequencer|Player|Play (Variables|/Script/LevelSequence.LevelSequenceActor|GetSequencePlayer _outactor) :!class /Script/MovieScene.MovieSceneSequencePlayer)
  (Variables|Default|SetActive_Sequence (Variables|/Script/LevelSequence.LevelSequenceActor|GetSequencePlayer _outactor))
  (Utilities|FlowControl|Delay 5.0)
  (Variables|Default|SetCamMoving false))

(event EventBeginPlay
  (Utilities|FlowControl|Sequence
    (:then_0
      (Utilities|Array|Clear (Variables|GamePlacements|GetFirst%20Place%20Array))
      (Utilities|Array|Add (Variables|GamePlacements|GetFirst%20Place%20Array) (Variables|GamePlacements|GetFirst%20Place%20G1))
      (Utilities|Array|Add (Variables|GamePlacements|GetFirst%20Place%20Array) (Variables|GamePlacements|GetFirst%20Place%20G2))
      (Utilities|Array|Add (Variables|GamePlacements|GetFirst%20Place%20Array) (Variables|GamePlacements|GetFirst%20Place%20G3))
      (Utilities|Array|Add (Variables|GamePlacements|GetFirst%20Place%20Array) (Variables|GamePlacements|GetFirst%20Place%20G4))
      (Utilities|Array|Add (Variables|GamePlacements|GetFirst%20Place%20Array) (Variables|GamePlacements|GetFirst%20Place%20G5))
      (Utilities|Array|Add (Variables|GamePlacements|GetFirst%20Place%20Array) (Variables|GamePlacements|GetFirst%20Place%20G6))
      (Utilities|Array|Add (Variables|GamePlacements|GetFirst%20Place%20Array) (Variables|GamePlacements|GetFirst%20Place%20G7)))
    (:then_1
      (Utilities|Array|Clear (Variables|GamePlacements|GetSecond%20Place%20Array))
      (Utilities|Array|Add (Variables|GamePlacements|GetSecond%20Place%20Array) (Variables|GamePlacements|GetSecond%20Place%20G1))
      (Utilities|Array|Add (Variables|GamePlacements|GetSecond%20Place%20Array) (Variables|GamePlacements|GetSecond%20Place%20G2))
      (Utilities|Array|Add (Variables|GamePlacements|GetSecond%20Place%20Array) (Variables|GamePlacements|GetSecond%20Place%20G3))
      (Utilities|Array|Add (Variables|GamePlacements|GetSecond%20Place%20Array) (Variables|GamePlacements|GetSecond%20Place%20G4))
      (Utilities|Array|Add (Variables|GamePlacements|GetSecond%20Place%20Array) (Variables|GamePlacements|GetSecond%20Place%20G5))
      (Utilities|Array|Add (Variables|GamePlacements|GetSecond%20Place%20Array) (Variables|GamePlacements|GetSecond%20Place%20G6))
      (Utilities|Array|Add (Variables|GamePlacements|GetSecond%20Place%20Array) (Variables|GamePlacements|GetSecond%20Place%20G7)))
    (:then_2
      (Utilities|Array|Clear (Variables|GamePlacements|GetThird%20Place%20Array))
      (Utilities|Array|Add (Variables|GamePlacements|GetThird%20Place%20Array) (Variables|GamePlacements|GetThird%20Place%20G1))
      (Utilities|Array|Add (Variables|GamePlacements|GetThird%20Place%20Array) (Variables|GamePlacements|GetThird%20Place%20G2))
      (Utilities|Array|Add (Variables|GamePlacements|GetThird%20Place%20Array) (Variables|GamePlacements|GetThird%20Place%20G3))
      (Utilities|Array|Add (Variables|GamePlacements|GetThird%20Place%20Array) (Variables|GamePlacements|GetThird%20Place%20G4))
      (Utilities|Array|Add (Variables|GamePlacements|GetThird%20Place%20Array) (Variables|GamePlacements|GetThird%20Place%20G5))
      (Utilities|Array|Add (Variables|GamePlacements|GetThird%20Place%20Array) (Variables|GamePlacements|GetThird%20Place%20G6))
      (Utilities|Array|Add (Variables|GamePlacements|GetThird%20Place%20Array) (Variables|GamePlacements|GetThird%20Place%20G7)))
    (:then_3
      (CallFunction|SetCode))
    (:then_4
      (CallFunction|GetData)
      (CallFunction|ApplyData))
    (:then_6
      (Variables|Default|SetNumberofGames_Int (Math|Conversions|ToInteger(Byte) (Utilities|String|ToString(Text) (Variables|GamePlacements|GetNumberofGames))))
      (if (>= (Variables|Default|GetNumberofGames_Int) 8)
        (Variables|Default|SetNumberofGames_Int 7)
        (Variables|GamePlacements|SetNumberofGames (Utilities|Text|ToText(Integer) 0))
        (elif (<= (Variables|Default|GetNumberofGames_Int) 0)
          (bind _output_get (Variables|Default|SetNumberofGames_Int 1))
          (Variables|GamePlacements|SetNumberofGames (Utilities|Text|ToText(Integer) _output_get))))
      (for _array_element (Actor|GetAllChildActors (Utilities|ResolveSoftReference (Variables|Blueprints|GetGames)) true)
        (Utilities|IsValid _array_element
          (:Is%20Valid
            (Actor|DestroyActor _array_element))))
      (if (not (<= (- (Variables|Default|GetNumberofGames_Int) 1) -1))
        (Variables|Default|SetRelative%20Transform (Math|Transform|MakeTransform (Math|Vector|MakeVector (Math|Conversions|ToFloat(Integer) (- -85 (/ (* (Variables|Default|GetNumberofGames_Int) 170) 2))) 0.0 0.0) "0, 0, 0" "1,1,1"))
        (for _index (range 0 (- (Variables|Default|GetNumberofGames_Int) 1))
          (Utilities|FlowControl|Sequence
            (:then_0
              (Variables|GamePlacements|SetFirst%20Place (Utilities|Array|Get(acopy) (Variables|GamePlacements|GetFirst%20Place%20Array) _index)))
            (:then_1
              (Variables|GamePlacements|SetSecond%20Place (Utilities|Array|Get(acopy) (Variables|GamePlacements|GetSecond%20Place%20Array) _index)))
            (:then_2
              (Variables|GamePlacements|SetThird%20Place (Utilities|Array|Get(acopy) (Variables|GamePlacements|GetThird%20Place%20Array) _index)))
            (:then_3
              (Variables|Default|SetRelative%20Transform (Math|Transform|MakeTransform (Math|Vector|MakeVector (+ (.x (.location (Variables|Default|GetRelative%20Transform))) 1.7e+02) 0.0 0.0) "0, 0, 0" "1,1,1"))
              (bind _returnvalue (AddComponent|AddChildActorComponent (Utilities|ResolveSoftReference (Variables|Blueprints|GetGames)) false (Variables|Default|GetRelative%20Transform)))
              (ChildActorComponent|SetChildActorClass _returnvalue "/Game/EFVS/Assets/Blueprints/BP_GamePanel_Top3.BP_GamePanel_Top3_C"))))))))

(fn ConstructionScript
  (CallFunction|Update)
  (Utilities|FlowControl|Sequence
    (:then_0
      (CallFunction|SetCode))
    (:then_1
      (CallFunction|GetData)
      (CallFunction|ApplyData))))

(fn CasterstoHost)